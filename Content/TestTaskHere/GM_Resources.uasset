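; Game mode that tracks the player's resource count, shows it on the HUD and persists it along with placed units.
; BeginPlay creates W_HUD, then loads the "Save" slot and respawns each A_Unit from its saved cost, mesh and transform.
; ChangeResources subtracts the given amount, refreshes the HUD and autosaves by rebuilding the save from all live units.
; ResetGame zeroes resources, destroys all units and saves through the same function.
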(event `self.ReceiveBeginPlay`
  (bind _returnvalue (`|CreateWidget` "/Game/TestTaskHere/W_HUD.W_HUD_C" (`GameplayStatics.GetPlayerController` 0)))
  (bind _output_get (set `self.PlayerHUD` _returnvalue))
  (`UserWidget.AddToViewport` _returnvalue 0)
  (`UserWidget.AddToViewport` _output_get 0)
  (bind _returnvalue_2 (`GameplayStatics.LoadGameFromSlot` "Save"))
  (bind _asbp_save (cast `/Game/TestTaskHere/BP_Save` _returnvalue_2))
  (set `self.Resource` (`/Game/TestTaskHere/BP_Save.ResourcesSave` _asbp_save))
  (for (_array_element _array_index) (`/Game/TestTaskHere/BP_Save.Units` _asbp_save)
    (`|SpawnActorFromClass` "/Game/TestTaskHere/A_Unit.A_Unit_C" (`|GetArrayItem` (`/Game/TestTaskHere/BP_Save.UnitTransforms` _asbp_save) _array_index) "Undefined" "MultiplyWithRoot" null (`.Cost_8_707431164701C35ED9DFE294BB3FAFEF` (break `/Game/TestTaskHere/Struct_Unit` _array_element)) (`.MeshData_12_EA3406C049D7BC0E8F4FAC81947E467F` (break `/Game/TestTaskHere/Struct_Unit` _array_element)) null))
  (`self.Change Resources` 0))

(event `Save Game`
  (bind _returnvalue (`GameplayStatics.CreateSaveGameObject` "/Game/TestTaskHere/BP_Save.BP_Save_C"))
  (bind _output_get (set `self.Save` _returnvalue))
  (set `/Game/TestTaskHere/BP_Save.ResourcesSave` (`self.Resource`) _output_get)
  (bind _outactors (`GameplayStatics.GetAllActorsOfClass` "/Game/TestTaskHere/A_Unit.A_Unit_C"))
  (for _array_element _outactors
    (`KismetArrayLibrary.Array_Add` (`/Game/TestTaskHere/BP_Save.Units` _output_get) (make `/Game/TestTaskHere/Struct_Unit` null "" (`/Game/TestTaskHere/A_Unit.Cost` _array_element) (`/Game/TestTaskHere/A_Unit.Mesh` _array_element)))
    (`KismetArrayLibrary.Array_Add` (`/Game/TestTaskHere/BP_Save.UnitTransforms` _output_get) (`self.GetTransform` _array_element)))
  (`GameplayStatics.SaveGameToSlot` _output_get "Save"))

(event `Reset Game`
  (set `self.Resource` 0)
  (bind _outactors (`GameplayStatics.GetAllActorsOfClass` "/Game/TestTaskHere/A_Unit.A_Unit_C"))
  (for _array_element _outactors
    (`self.K2_DestroyActor` _array_element))
  (`self.Change Resources` 0))

(fn `Change Resources`
  (params (Change :type Integer))
  (set `self.Resource` (- (`self.Resource`) Change))
  (`/Game/TestTaskHere/W_HUD.Update Resources` (`self.PlayerHUD`))
  (`self.Save Game`))

(fn `UserConstructionScript`)